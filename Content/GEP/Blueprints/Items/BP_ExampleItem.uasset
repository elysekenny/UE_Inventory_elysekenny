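; BP_ExampleItem is an example pickup item actor whose item data is based on its colour.
; The construction script applies the item model to the mesh, and BeginPlay builds the colour data through InitColour.
; Its Pickup event adds that data to the player's InventorySystem and destroys the actor only if the add succeeds.
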(event EventBeginPlay
  (bind _colourdata (CallFunction|InitColour)) ; sets the width and height based on the item
  (Variables|Default|SetColour%20Data _colourdata))

(event EventPickup
  (params (Item :type Actor%20Class%20Reference) (Player :type BP%20Player%20Character%20Object%20Reference))
  (bind _success (Default|AddItem (Variables|/Game/GEP/Blueprints/Essentials/BP_PlayerCharacter.BP_PlayerCharacter_C|GetInventory_System Player) (Variables|Default|GetColour%20Data)))
  (if _success
    (Actor|DestroyActor)))

(fn ConstructionScript
  (Components|StaticMesh|SetStaticMesh (Variables|Default|GetMesh) (Variables|Default|GetItem_model)))

(fn InitColour
  (Default|Init (Variables|Default|GetItemData) (Variables|Default|GetItemColour)) ; sets the height and width based on the colour
)

(fn GetColour
  (return (Variables|Default|GetItemColour)))