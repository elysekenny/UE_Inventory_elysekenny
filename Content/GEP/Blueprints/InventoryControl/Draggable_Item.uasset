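; Draggable_Item describes an inventory item by colour, slot colour, icon, width and height, exposed through simple getters.
; GetItemActor switches on Colour to return the matching item: Red, Blue, Yellow, Green, Orange or Purple, with BP_ExampleItem as the fallback.
; Its comment mentions a data table row name, but the selection uses only the Colour value.
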(fn GetColour
  (return (Variables|Default|GetColour)))

(fn GetWidth
  (return (Variables|Default|GetWidth)))

(fn GetHeight
  (return (Variables|Default|GetHeight)))

(fn GetIcon
  (return (Variables|Default|GetIcon)))

(fn GetSlotColour
  (return (Variables|Default|GetSlot_Colour)))

(fn GetItemActor
  ;[0.04382 0.2188 0] Retrieves the actual item to be displayed based on the data table row name
  (switch name (Variables|Default|GetColour)
    (:Default
      (LocalVariables|SetItemColour "/Game/GEP/Blueprints/Items/BP_ExampleItem.BP_ExampleItem_C"))
    (:Red
      (LocalVariables|SetItemColour "/Game/GEP/Blueprints/Items/Red_Item.Red_Item_C"))
    (:Blue
      (LocalVariables|SetItemColour "/Game/GEP/Blueprints/Items/Blue_Item.Blue_Item_C"))
    (:Yellow
      (LocalVariables|SetItemColour "/Game/GEP/Blueprints/Items/Yellow_Item.Yellow_Item_C"))
    (:Green
      (LocalVariables|SetItemColour "/Game/GEP/Blueprints/Items/Green_Item.Green_Item_C"))
    (:Orange
      (LocalVariables|SetItemColour "/Game/GEP/Blueprints/Items/Orange_Item.Orange_Item_C"))
    (:Purple
      (LocalVariables|SetItemColour "/Game/GEP/Blueprints/Items/Purple_Item.Purple_Item_C")))
  (return (LocalVariables|GetItemColour)))