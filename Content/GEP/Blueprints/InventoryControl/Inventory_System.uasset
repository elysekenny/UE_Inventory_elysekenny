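; Grid inventory system that stores items of varying width and height across tiles in a flat array.
; AddItem scans for the first spot where every covered tile is in bounds and empty, then fills those tiles; RemoveItem clears all tiles matching the item's row name.
; Changes set a dirty flag, so Tick fires OnInventoryChanged only when needed.
; Helpers convert index to tile, list stored items and resolve slot data from a data table.
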(event EventBeginPlay
  (Utilities|Array|Resize (Variables|Default|GetItems) (* (Variables|Default|GetMaxWidth) (Variables|Default|GetMaxHeight))))

(event EventTick
  (params (DeltaSeconds :type Float%20%28single-precision%29))
  (if (Variables|Default|GetIsDirty)
    (Variables|Default|SetIsDirty false)
    (Default|CallOnInventoryChanged) ; only redraws the inventory when it has been changed as opposed to every frame
  ))

(event EventTransferItemData
  (params (ItemData :type Complete%20Item%20Data%20Structure))
  (Variables|Default|SetItemHovered ItemData))

(fn AddItem
  (params (ItemData :type Item%20Data%20Object%20Reference))
  (bind _output_get (Variables|Default|SetItemToAdd ItemData))
  (Utilities|IsValid _output_get
    (:Is%20Valid
      (for (_ _array_index) (Variables|Default|GetItems)
        (bind _foundslot (CallFunction|IsFreeSpace _array_index (Variables|Default|GetItemToAdd)))
        (if _foundslot
          (CallFunction|AddItematIndex (Variables|Default|GetItemToAdd) _array_index)
          (return true)))
      (return false))))

(fn RemoveItem
  (params (ItemToRemove :type Complete%20Item%20Data%20Structure))
  (LocalVariables|SetItem%20To%20Remove ItemToRemove)
  (for (_array_element _array_index) (Variables|Default|GetItems)
    (if (== (.itemname _array_element) (.rowname (LocalVariables|GetItem%20To%20Remove)))
      (Utilities|Array|SetArrayElem :TargetArray (Variables|Default|GetItems) :Index _array_index)
      (Variables|Default|SetIsDirty true))))

(fn IsFreeSpace
  (params (TopLeftIndex :type Integer) (ItemToCheck :type Item%20Data%20Object%20Reference))
  (Utilities|FlowControl|Sequence
    (:then_0
      (bind _tile (Utilities|ForEachIndex TopLeftIndex ItemToCheck)
        (:LoopBody
          (Utilities|IsTileValid _tile
            (:true
              (bind (_valid _item_name) (CallFunction|GetItematIndex (CallFunction|TiletoIndex _tile)))
              (if _valid
                (if (!= _item_name "")
                  (return false))
                (else
                  (return false))))
            (:false
              (return false))))))
    (:then_1
      (return true))))

(fn IndextoTile
  (params (Index :type Integer))
  (return (Utilities|Struct|MakeInventory_Tile (Math|Integer|%(Integer) Index (Variables|Default|GetMaxWidth)) (/ Index (Variables|Default|GetMaxWidth)))))

(fn GetItematIndex
  (params (Index :type Integer))
  (if (Utilities|Array|IsValidIndex (Variables|Default|GetItems) Index)
    (return true (.ItemName (Utilities|Struct|BreakF_Slot_Structure (Utilities|Array|Get(acopy) (Variables|Default|GetItems) Index))))
    (else
      (return false "None"))))

(fn TiletoIndex
  (params (Tile :type Inventory%20Tile%20Structure))
  (bind (_x _y) (Utilities|Struct|BreakInventory_Tile Tile))
  (return (+ _x (* _y (Variables|Default|GetMaxWidth)))))

(fn GetAllItems
  (params (InventorySystem :type Inventory%20System%20Object%20Reference))
  (LocalVariables|SetCurrentSystem InventorySystem)
  (for (_array_element _array_index) (Variables|Default|GetItems)
    (LocalVariables|SetCurrentSlotData _array_element)
    (if (not (Utilities|Map|Contains (LocalVariables|GetAllItems%28Local%29) _array_element))
      (Utilities|Map|Add (LocalVariables|GetAllItems%28Local%29) (LocalVariables|GetCurrentSlotData) (CallFunction|IndextoTile (LocalVariables|GetCurrentSystem) _array_index))))
  (return (LocalVariables|GetAllItems%28Local%29)))

(fn GetDatafromSlot
  (params (Slot :type F%20Slot%20Structure%20Structure))
  (bind _returnvalue (Utilities|GetDataTableRow "/Game/GEP/Blueprints/InventoryControl/Items.Items" (.itemname Slot)) ; item colour corresponds to the row name
    (:then
      (bind _output_get (Variables|Default|SetItemDataConverted (Utilities|Struct|MakeCompleteItemData (.itemname Slot) (.itemname _returnvalue) (.itemdescription _returnvalue) (.icon _returnvalue) (.slotcolour _returnvalue) (.width _returnvalue) (.height _returnvalue))))
      (return _output_get true))
    (:RowNotFound
      (return "" false))))

(fn AddItematIndex
  (params (ItemToAdd :type Item%20Data%20Object%20Reference) (Index :type Integer))
  (bind _output_get (LocalVariables|SetLocalItemData ItemToAdd))
  (bind _tile (Utilities|ForEachIndex Index _output_get)
    (:LoopBody
      (Utilities|Array|SetArrayElem (Variables|Default|GetItems) (CallFunction|TiletoIndex _tile) (Utilities|Struct|MakeF_Slot_Structure (.RowName (Utilities|Struct|BreakDataTableRowHandle (Variables|/Game/GEP/Blueprints/InventoryControl/ItemData.ItemData_C|GetRowName (LocalVariables|GetLocalItemData)))) (Variables|/Game/GEP/Blueprints/InventoryControl/ItemData.ItemData_C|GetWidth (LocalVariables|GetLocalItemData)) (Variables|/Game/GEP/Blueprints/InventoryControl/ItemData.ItemData_C|GetHeight (LocalVariables|GetLocalItemData)))))
    (:Completed
      (Variables|Default|SetIsDirty true) ; flag for changes
    )))